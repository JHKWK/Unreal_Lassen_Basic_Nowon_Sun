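; BP_Slime is a player-controlled slime character with forward-axis movement, yaw turning and a hold-to-sprint input.
; Movement input follows player controller 0's actor forward vector, while yaw input to that controller is scaled by YawSpeed and frame delta time.
; Sprint press and release switch the CharacterMovement max walk speed between fast and normal values, with normal set on BeginPlay.
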(event EventBeginPlay
  (Variables|/Script/Engine.CharacterMovementComponent|SetMaxWalkSpeed (Variables|Character|GetCharacterMovement) 6e+02))

(event Collision|EventActorBeginOverlap
  (params (OtherActor :type Actor%20Object%20Reference)))

(event EventTick
  (params (DeltaSeconds :type Float%20%28single-precision%29)))

(event Input|ActionEvents|InputActionOnSprint
  (params (Key :type Key%20Structure :default "None"))
  (:Pressed
    (Variables|/Script/Engine.CharacterMovementComponent|SetMaxWalkSpeed (Variables|Character|GetCharacterMovement) 2e+03))
  (:Released
    (Variables|/Script/Engine.CharacterMovementComponent|SetMaxWalkSpeed (Variables|Character|GetCharacterMovement) 6e+02)))

(event Input|AxisEvents|InputAxisONMoveForward
  (params (AxisValue :type Float%20%28single-precision%29))
  (Pawn|Input|AddMovementInput (Transformation|GetActorForwardVector (Game|GetPlayerController 0)) AxisValue false))

(event Input|AxisEvents|InputAxisOnYaw
  (params (AxisValue :type Float%20%28single-precision%29))
  (Class|PlayerController|AddYawInput (Game|GetPlayerController 0) (* (* AxisValue (Variables|Default|GetYawSpeed)) (Utilities|Time|GetWorldDeltaSeconds))))

(fn ConstructionScript)