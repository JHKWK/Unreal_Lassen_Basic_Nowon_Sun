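; BP_PWN_Camera_InvenLIst is a pawn Blueprint that lets the player click items in the world to send their info to the list inventory.
; On left mouse release, a visibility trace under the cursor looks for an actor tagged "Item" and casts it to BP_Item.
; The item's Info goes to MpDXinventory's BuildListWithInfo, and its ID, name and description are printed as colored debug text.
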(event EventBeginPlay)

(event Collision|EventActorBeginOverlap
  (params (OtherActor :type Actor%20Object%20Reference)))

(event EventTick
  (params (DeltaSeconds :type Float%20%28single-precision%29)))

(event Input|MouseEvents|LeftMouseButton
  (params (Key :type Key%20Structure))
  (bind _returnvalue (Game|GetPlayerController 0))
  (bind (_hitresult _returnvalue_2) (Game|Player|GetHitResultUnderCursorbyChannel _returnvalue "TraceTypeQuery1" true))
  (bind (_bblockinghit _binitialoverlap _time _distance _location _impactpoint _normal _impactnormal _physmat _hitactor) (Collision|BreakHitResult _hitresult))
  (:Released
    (if _returnvalue_2
      (if _bblockinghit
        (if (Actor|ActorHasTag _hitactor "Item")
          (bind _asbp_item (Utilities|Casting|CastToBP_Item _hitactor))
          (Default|BuildListwithInfo (Variables|Default|GetmpDXinventory) (Variables|/Game/LIstInventory/BP_Item.BP_Item_C|GetInfo _asbp_item))
          (Development|PrintText (Utilities|Text|FormatText "ID : {_id}  Name:{_name}   Info:{_info}" (.mIndex (Utilities|Struct|BreakST_ItemInfo (Variables|/Game/LIstInventory/BP_Item.BP_Item_C|GetInfo _asbp_item))) (.mName (Utilities|Struct|BreakST_ItemInfo (Variables|/Game/LIstInventory/BP_Item.BP_Item_C|GetInfo _asbp_item))) (.mInfo (Utilities|Struct|BreakST_ItemInfo (Variables|/Game/LIstInventory/BP_Item.BP_Item_C|GetInfo _asbp_item)))) true true "(R=1.000000,G=0.401789,B=0.471593,A=1.000000)"))))))

(fn ConstructionScript)