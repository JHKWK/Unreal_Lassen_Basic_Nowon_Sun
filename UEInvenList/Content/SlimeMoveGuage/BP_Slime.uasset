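; Player-controlled slime actor that moves, jumps and picks up items to feed an EXP gauge UI.
; Forward and yaw axis inputs share one frame-time-scaled world transform node for moving and turning.
; Timelines drive squash-and-stretch mesh scaling and set jump height as absolute Z, with IsJumping blocking re-jumps.
; Overlapping a BP_Item prints a Korean pickup message and passes an item info value to the gauge.
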(event EventBeginPlay)

(event Collision|EventActorBeginOverlap
  (params (OtherActor :type Actor%20Object%20Reference))
  (bind _asbp_item (Utilities|Casting|CastToBP_Item OtherActor))
  (Development|PrintText (Utilities|Text|FormatText "{_name}(을)를 얻었다" (.mname (Variables|/Game/LIstInventory/BP_Item.BP_Item_C|GetInfo _asbp_item))))
  (Default|BuildUI (Variables|Default|GetmpUIGuageEXP) (.membervar_10 (Variables|/Game/LIstInventory/BP_Item.BP_Item_C|GetInfo _asbp_item))))

(event EventTick
  (params (DeltaSeconds :type Float%20%28single-precision%29))
  (if (not (Variables|Default|GetisJumping))
    (bind (_direction _newtrack_0 _newtrack_1) (Timeline|Timeline_0 Play)
      (:Update
        (Transformation|SetRelativeScale3D (Variables|Default|GetStaticMesh) (Math|Vector|MakeVector _newtrack_1 _newtrack_0 _newtrack_1))))))

(event Input|ActionEvents|InputActionOnJump
  (params (Key :type Key%20Structure :default "None"))
  (bind _returnvalue (Transformation|GetActorLocation))
  (:Pressed
    (if (not (Variables|Default|GetisJumping))
      (bind (_direction _newtrack_0 _newtrack_2) (Timeline|Timeline_1 PlayFromStart)
        (:Update
          (Variables|Default|SetisJumping true)
          (Transformation|SetActorLocation (Math|Vector|MakeVector (.x _returnvalue) (.y _returnvalue) _newtrack_0) false false)
          (Transformation|SetRelativeScale3D (Variables|Default|GetStaticMesh) (Math|Vector|MakeVector 1.0 _newtrack_2 1.0)))
        (:Finished
          (Variables|Default|SetisJumping false))))))

(event Input|AxisEvents|InputAxisOnMoveForward
  (params (AxisValue :type Float%20%28single-precision%29))
  (Class|Actor|AddActorWorldTransform (Math|Transform|MakeTransform (* (* (* (Transformation|GetActorForwardVector) AxisValue) (Variables|Default|GetSpeed)) (Utilities|Time|GetWorldDeltaSeconds)) (Math|Rotator|MakeRotator 0.0 0.0 (* (* (stale Input|AxisEvents|InputAxisOnRotateYaw AxisValue) (Variables|Default|GetRotateSpeed)) (Utilities|Time|GetWorldDeltaSeconds))) "0.000000,0.000000,0.000000") false false))

(event Input|AxisEvents|InputAxisOnRotateYaw
  (params (AxisValue :type Float%20%28single-precision%29))
  (Class|Actor|AddActorWorldTransform (Math|Transform|MakeTransform (* (* (* (Transformation|GetActorForwardVector) (stale Input|AxisEvents|InputAxisOnMoveForward AxisValue)) (Variables|Default|GetSpeed)) (Utilities|Time|GetWorldDeltaSeconds)) (Math|Rotator|MakeRotator 0.0 0.0 (* (* AxisValue (Variables|Default|GetRotateSpeed)) (Utilities|Time|GetWorldDeltaSeconds))) "0.000000,0.000000,0.000000") false false))

(fn ConstructionScript)