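; BP_PwnCamera is a camera pawn that lets the player pick up items with the mouse.
; On left mouse release it traces the Visibility channel under the cursor for an actor tagged "tagItem".
; It stores that actor, casts it to BP_Item to pass its MItemInfo to MpUiONPlay's BuildUI, then destroys it.
; An unconnected debug chain would print the item's name and description.
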(event EventBeginPlay)

(event Collision|EventActorBeginOverlap
  (params (OtherActor :type Actor%20Object%20Reference)))

(event EventTick
  (params (DeltaSeconds :type Float%20%28single-precision%29)))

(event Input|MouseEvents|LeftMouseButton
  (params (Key :type Key%20Structure :default "None"))
  (bind _returnvalue (Game|GetPlayerController 0))
  (bind (_hitresult _returnvalue_2) (Game|Player|GetHitResultUnderCursorbyChannel _returnvalue "TraceTypeQuery1" false))
  (bind _hitactor (Collision|BreakHitResult _hitresult))
  (:Released
    (if _returnvalue_2
      (if (Actor|ActorHasTag _hitactor "tagItem")
        (Variables|Default|SetBPItem _hitactor)
        (Utilities|FlowControl|Sequence
          (:then_1
            (bind _asbp_item (Utilities|Casting|CastToBP_Item (Variables|Default|GetBPItem)))
            (Default|BuildUI (Variables|Default|GetmpUiONPlay) (Variables|/Game/BP_Item.BP_Item_C|GetmItemInfo _asbp_item)))
          (:then_2
            (Actor|DestroyActor (Variables|Default|GetBPItem))))))))

(fn ConstructionScript)