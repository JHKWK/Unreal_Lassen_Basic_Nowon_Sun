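; BP_PWNCamera handles click-to-shoot scoring, judging whether the player clicked an enemy.
; On left mouse release, it traces Visibility under the cursor and checks the hit actor for the "Enemy" tag.
; Enemy hits increment MScore in BP_GameInstance and print Korean hit and score messages, while other hit actors print a taunt.
; Every release then calls the EvtOnMouseClick dispatcher; older local Score logic remains unconnected.
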(event EventBeginPlay)

(event Collision|EventActorBeginOverlap
  (params (OtherActor :type Actor%20Object%20Reference)))

(event EventTick
  (params (DeltaSeconds :type Float%20%28single-precision%29)))

(event Input|MouseEvents|LeftMouseButton
  (params (Key :type Key%20Structure :default "None"))
  (bind _returnvalue (Game|GetPlayerController 0))
  (bind (_hitresult _returnvalue_2) (Game|Player|GetHitResultUnderCursorbyChannel _returnvalue "TraceTypeQuery1" true))
  (:Released
    (Utilities|FlowControl|Sequence
      (:then_1
        (if _returnvalue_2
          (if (Actor|ActorHasTag (.HitActor (Collision|BreakHitResult _hitresult)) "Enemy")
            (Development|PrintString "명중!!" true true "(R=1.000000,G=0.913893,B=0.000000,A=1.000000)")
            (bind _asbp_game_instance (Utilities|Casting|CastToBP_GameInstance (Game|GetGameInstance)))
            (bind _result (Math|Integer|IncrementInt (Variables|/Game/BP_GameInstance.BP_GameInstance_C|GetmScore _asbp_game_instance))
              (:%20%20
                (Development|PrintText (Utilities|Text|FormatText "현재 스코어 : {score}" _result) true true "(R=0.043461,G=1.000000,B=0.000000,A=1.000000)")))
            (else
              (Development|PrintText "그건 제 잔상입니다만?" true true "(R=1.000000,G=0.030746,B=0.366305,A=1.000000)")))))
      (:then_2
        (Default|CallEvtonMouseClick)))))

(fn ConstructionScript)