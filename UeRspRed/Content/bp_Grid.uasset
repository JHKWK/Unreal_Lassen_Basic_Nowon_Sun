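; Scrolling grid actor that moves three blocks along negative X in an endless loop.
; BeginPlay records each block's starting position and spawns a wolf pawn attached to a socket on Block2.
; Tick shifts the blocks by speed times delta time, snapping any that pass the X threshold to the last block's original position.
; StopScroll zeroes the speed and switches the scroll state to halt movement.
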(event EventBeginPlay
  (Utilities|FlowControl|Sequence
    (:then_0
      (for _array_element (Variables|Default|GetmBlocks)
        (Utilities|Array|Add (Variables|Default|GetmOriginalLocation) (Variables|/Script/Engine.SceneComponent|GetRelativeLocation _array_element))))
    (:then_1
      (bind _returnvalue (Game|SpawnActorfromClass "/Game/pwn_Wolf.pwn_Wolf_C" (Math|Transform|MakeTransform "0, 0, 0" "0,180.000000, 0") "Undefined" 0 0))
      (Transformation|AttachComponentToComponent _returnvalue (Variables|Default|Getblock2) "Socket" "KeepRelative" "KeepRelative" "KeepRelative" true))))

(event Collision|EventActorBeginOverlap
  (params (OtherActor :type Actor%20Object%20Reference)))

(event EventTick
  (params (DeltaSeconds :type Float%20%28single-precision%29))
  (CallFunction|UpdateScroll))

(fn ConstructionScript
  (Utilities|Array|Add (Variables|Default|GetmBlocks) (Variables|Default|Getblock0))
  (Utilities|Array|Add (Variables|Default|GetmBlocks) (Variables|Default|Getblock1))
  (Utilities|Array|Add (Variables|Default|GetmBlocks) (Variables|Default|Getblock2))
  (Variables|Default|SetmScrollState "NewEnumerator0"))

(fn UpdateScroll
  (switch Utilities|FlowControl|Switch|Switchonen_BlockScroll (Variables|Default|GetmScrollState)
    (:NewEnumerator0
      (bind _output_get (LocalVariables|SettLastIndex (- (Utilities|Array|Length (Variables|Default|GetmBlocks)) 1)))
      (for _index (range 0 _output_get)
        (LocalVariables|SettIndex _index)
        (Utilities|FlowControl|Sequence
          (:then_0
            ;[1 1 1] Comment
            (Transformation|SetRelativeLocation (Utilities|Array|Get(acopy) (Variables|Default|GetmBlocks) (LocalVariables|GettIndex)) (Math|Vector|MakeVector (+ (.x (Variables|/Script/Engine.SceneComponent|GetRelativeLocation (Utilities|Array|Get(acopy) (Variables|Default|GetmBlocks) (LocalVariables|GettIndex)))) (* (Variables|Default|GetmSpeedScroll) (Utilities|Time|GetWorldDeltaSeconds) -1.0)) 0.0 0.0) false false))
          (:then_1
            ;[1 1 1] Comment
            (if (<= (.x (Variables|/Script/Engine.SceneComponent|GetRelativeLocation (Utilities|Array|Get(acopy) (Variables|Default|GetmBlocks) (LocalVariables|GettIndex)))) -9.8e+02)
              (Transformation|SetRelativeLocation (Utilities|Array|Get(acopy) (Variables|Default|GetmBlocks) (LocalVariables|GettIndex)) (Utilities|Array|Get(acopy) (Variables|Default|GetmOriginalLocation) (LocalVariables|GettLastIndex)) false false))))))))

(fn StopScroll
  (Variables|Default|SetmSpeedScroll 0.0)
  (Variables|Default|SetmScrollState "NewEnumerator1"))